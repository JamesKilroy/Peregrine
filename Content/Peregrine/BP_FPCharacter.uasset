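; First-person player character that hosts movement, physics grab, tether pulling and inventory components, and creates the controls and quick-slot HUDs.
; Input forwards to components for walking, jumping, mantling, wall-running, tethering, and grabbing, rotating, zooming or throwing objects.
; Look input pauses camera during rotation mode, while middle mouse polls through a gate to lock rotation to one axis.
; A far trigger starts overlapped actors' inventories; a spawn chain swaps actors for grabbable objects.
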(event OnComponentBeginOverlap(TriggerRangeFar)
  (params (OverlappedComponent :type Primitive%20Component%20Object%20Reference) (OtherActor :type Actor%20Object%20Reference) (OtherComp :type Primitive%20Component%20Object%20Reference) (OtherBodyIndex :type Integer) (bFromSweep :type Boolean) (SweepResult :type Hit%20Result%20Structure%20%28by%20ref%29))
  (Development|PrintString (Utilities|GetDisplayName OtherActor))
  (bind _component (Class|IInventory|GetInventoryComponent(Message) OtherActor))
  (Utilities|IsValid _component
    (:Is%20Valid
      (Development|PrintString "valid")
      (Class|ACInventory|StartComponent _component false))))

(event OnComponentEndOverlap(TriggerRangeFar)
  (params (OverlappedComponent :type Primitive%20Component%20Object%20Reference) (OtherActor :type Actor%20Object%20Reference) (OtherComp :type Primitive%20Component%20Object%20Reference) (OtherBodyIndex :type Integer)))

(event Custom|LookUp
  (params (LookUp :type Float%20%28double-precision%29))
  ;[0.15 0.1095 0.01756 0.5] Grab System
  ;;[1 0.6517 0.3191] Set Axis
  (Variables|Default|SetLookUp%20Axis%20Value LookUp))

(event Custom|Turn
  (params (Turn :type Float%20%28double-precision%29))
  ;[0.15 0.1095 0.01756 0.5] Grab System
  ;;[1 0.6517 0.3191] Set Axis
  (Variables|Default|SetTurn%20Axis%20Value Turn))

(event Custom|Unlimit%20Rotation
  (bind _turn_axis_value (Variables|Default|GetTurn%20Axis%20Value))
  (bind _lookup_axis_value (Variables|Default|GetLookUp%20Axis%20Value))
  ;[0.15 0.1095 0.01756 0.5] Grab System
  ;;[1 0.6517 0.3191] Limit Rotation Direction Logic
  (Utilities|FlowControl|Sequence
    (:then_0
      (Utilities|FlowControl|Gate true) ; enters at Open
    )
    (:then_1
      (Default|DisableRotationAxes (Variables|Default|GetAC_GrabSystem) false false))))

(event Custom|Limit%20Rotation
  (bind _turn_axis_value (Variables|Default|GetTurn%20Axis%20Value))
  (bind _lookup_axis_value (Variables|Default|GetLookUp%20Axis%20Value))
  ;[0.15 0.1095 0.01756 0.5] Grab System
  ;;[1 0.6517 0.3191] Limit Rotation Direction Logic
  (Variables|/Game/GrabSystem/Blueprint/ActorComponent/AC_GrabSystem.AC_GrabSystem_C|GetAs%20BP%20Master%20Grab (Variables|Default|GetAC_GrabSystem)
    (:then
      (Utilities|FlowControl|Sequence
        (:then_0
          (goto _label Open))
        (:then_1
          (Utilities|FlowControl|Gate true :!label _label
            (:Exit
              (if (or (Math|Float|InRange(Float) _lookup_axis_value 0.2 1.0) (Math|Float|InRange(Float) _lookup_axis_value -1.0 -0.2))
                (Default|DisableRotationAxes (Variables|Default|GetAC_GrabSystem) false true)
                (goto _label Close)
                (elif (or (Math|Float|InRange(Float) _turn_axis_value 0.2 1.0) (Math|Float|InRange(Float) _turn_axis_value -1.0 -0.2))
                  (Default|DisableRotationAxes (Variables|Default|GetAC_GrabSystem) true false)
                  (goto _label Close)
                  (else
                    (Utilities|FlowControl|Delay 0.05)
                    (goto _label)))))))))
    (:else)))

(event Custom|SpawnActorServer
  (params (SpawnActorInfos :type F%20Spawn%20Actor%20Infos%20Structure))
  (bind (_spawnactortranformref _mustdestroyactor) (Utilities|Struct|BreakF_SpawnActorInfos SpawnActorInfos))
  ;[0.15 0.1095 0.01756 0.5] Grab System
  ;;[1 0.6109 0.1818] Spawn actor logic
  (CallFunction|DestroyActorMulti _mustdestroyactor)
  (Utilities|FlowControl|Delay 0.0)
  (bind _returnvalue (Game|SpawnActorfromClass "/Game/GrabSystem/Blueprint/Actor/BP_Master_Grab.BP_Master_Grab_C" _spawnactortranformref "AlwaysSpawn" "OverrideRootScale" 0 false true true 0 false 0 0))
  (Default|NewStaticMeshServer _returnvalue SpawnActorInfos)
  (Utilities|FlowControl|Delay 0.0)
  (Default|InteractServer (Variables|Default|GetAC_GrabSystem)))

(event Custom|DestroyActorMulti
  (params (Actor :type Actor%20Object%20Reference))
  ;[0.15 0.1095 0.01756 0.5] Grab System
  ;;[1 0.6109 0.1818] Spawn actor logic
  (Actor|DestroyActor Actor))

(event Input|EnhancedActionEvents|EnhancedInputActionIA_Jump
  (params (ActionValue :type Boolean) (ElapsedSeconds :type Float%20%28double-precision%29) (TriggeredSeconds :type Float%20%28double-precision%29) (InputAction :type Input%20Action%20Object%20Reference :default "/Game/Peregrine/Input/IA_Jump.IA_Jump"))
  ;[0.03432 0.15 0.1465 0.5] Movement
  (:Started
    (Default|OnJump (Variables|Default|GetAC_FPMovement))))

(event Input|EnhancedActionEvents|EnhancedInputActionIA_Move
  (params (ActionValue :type Vector%202D%20Structure) (ElapsedSeconds :type Float%20%28double-precision%29) (TriggeredSeconds :type Float%20%28double-precision%29) (InputAction :type Input%20Action%20Object%20Reference :default "/Game/Peregrine/Input/IA_Move.IA_Move"))
  ;[0.03432 0.15 0.1465 0.5] Movement
  (Default|OnWalk (Variables|Default|GetAC_FPMovement) (.x ActionValue) (.y ActionValue)))

(event Input|EnhancedActionEvents|EnhancedInputActionIA_Look
  (params (ActionValue :type Vector%202D%20Structure) (ElapsedSeconds :type Float%20%28double-precision%29) (TriggeredSeconds :type Float%20%28double-precision%29) (InputAction :type Input%20Action%20Object%20Reference :default "/Game/Peregrine/Input/IA_Look.IA_Look"))
  ;[0.03432 0.15 0.1465 0.5] Movement
  (:Triggered
    ;;[0.15 0.15 0.15 0.5] Grab system input passthrough
    (CallFunction|Turn (.x ActionValue))
    (CallFunction|LookUp (.y ActionValue))
    (if (not (Variables|/Game/GrabSystem/Blueprint/ActorComponent/AC_GrabSystem.AC_GrabSystem_C|GetRotationMode (Variables|Default|GetAC_GrabSystem)))
      (Default|OnLook (Variables|Default|GetAC_FPMovement) (.x ActionValue) (.y ActionValue))))
  (:Completed
    (CallFunction|Turn 0.0)
    (CallFunction|LookUp 0.0)))

(event Input|EnhancedActionEvents|EnhancedInputActionIA_Mantle
  (params (ActionValue :type Boolean) (ElapsedSeconds :type Float%20%28double-precision%29) (TriggeredSeconds :type Float%20%28double-precision%29) (InputAction :type Input%20Action%20Object%20Reference :default "/Game/Peregrine/Input/IA_Mantle.IA_Mantle"))
  ;[0.03432 0.15 0.1465 0.5] Movement
  (:Started
    (Default|OnMantle (Variables|Default|GetAC_FPMovement))
    (Development|PrintString "Try mantle")))

(event Input|EnhancedActionEvents|EnhancedInputActionIA_Teather
  (params (ActionValue :type Boolean) (ElapsedSeconds :type Float%20%28double-precision%29) (TriggeredSeconds :type Float%20%28double-precision%29) (InputAction :type Input%20Action%20Object%20Reference :default "/Game/Peregrine/Input/IA_Teather.IA_Teather"))
  (bind _ac_pullingsystem (Variables|Default|GetAC_PullingSystem))
  ;[1 0.6517 0.3191] Pull System
  (:Started
    (Default|InteractServer _ac_pullingsystem))
  (:Completed
    (Default|EndInteractServer _ac_pullingsystem)))

(event Input|EnhancedActionEvents|EnhancedInputActionIA_UnTeather
  (params (ActionValue :type Boolean) (ElapsedSeconds :type Float%20%28double-precision%29) (TriggeredSeconds :type Float%20%28double-precision%29) (InputAction :type Input%20Action%20Object%20Reference :default "/Game/Peregrine/Input/IA_UnTeather.IA_UnTeather"))
  ;[1 0.6517 0.3191] Pull System
  (Default|DestroyAllPullingActors (Variables|Default|GetAC_PullingSystem))
  (Variables|Default|SetCurentPullPower (Variables|Default|GetDefaultPullPower)))

(event Input|EnhancedActionEvents|EnhancedInputActionIA_Run
  (params (ActionValue :type Boolean) (ElapsedSeconds :type Float%20%28double-precision%29) (TriggeredSeconds :type Float%20%28double-precision%29) (InputAction :type Input%20Action%20Object%20Reference :default "/Game/Peregrine/Input/IA_Run.IA_Run"))
  (bind _ac_fpmovement (Variables|Default|GetAC_FPMovement))
  ;[0.03432 0.15 0.1465 0.5] Movement
  (:Started
    (Default|OnRunStart _ac_fpmovement))
  (:Completed
    (Default|OnRunEnd _ac_fpmovement)))

(event Input|EnhancedActionEvents|EnhancedInputActionIA_Interact
  (params (ActionValue :type Boolean) (ElapsedSeconds :type Float%20%28double-precision%29) (TriggeredSeconds :type Float%20%28double-precision%29) (InputAction :type Input%20Action%20Object%20Reference :default "/Game/Peregrine/Input/IA_Interact.IA_Interact"))
  (bind _ac_grabsystem (Variables|Default|GetAC_GrabSystem))
  ;[0.15 0.1095 0.01756 0.5] Grab System
  ;;[0.15 0.15 0.15 0.5] Input
  ;;;[1 0.6517 0.3191] Grab
  (:Started
    (Variables|/Game/GrabSystem/Blueprint/ActorComponent/AC_GrabSystem.AC_GrabSystem_C|GetAs%20BP%20Master%20Grab _ac_grabsystem
      (:then)
      (:else
        (Default|InteractServer _ac_grabsystem))))
  (:Completed
    (Variables|/Game/GrabSystem/Blueprint/ActorComponent/AC_GrabSystem.AC_GrabSystem_C|GetAs%20BP%20Master%20Grab _ac_grabsystem
      (:then
        (Default|EndInteractServer _ac_grabsystem false 0.0))
      (:else))))

(event Input|EnhancedActionEvents|EnhancedInputActionIA_WallRun
  (params (ActionValue :type Boolean) (ElapsedSeconds :type Float%20%28double-precision%29) (TriggeredSeconds :type Float%20%28double-precision%29) (InputAction :type Input%20Action%20Object%20Reference :default "/Game/Peregrine/Input/IA_WallRun.IA_WallRun"))
  ;[0.03432 0.15 0.1465 0.5] Movement
  (:Started
    (Default|StartWallRun (Variables|Default|GetAC_FPMovement))
    (Development|PrintString "try wallrun" :!label _label))
  (:Completed
    (Default|StopWallRun (Variables|Default|GetAC_FPMovement))
    (goto _label)))

(event Input|EnhancedActionEvents|EnhancedInputActionIA_Throw
  (params (ActionValue :type Boolean) (ElapsedSeconds :type Float%20%28double-precision%29) (TriggeredSeconds :type Float%20%28double-precision%29) (InputAction :type Input%20Action%20Object%20Reference :default "/Game/Peregrine/Input/IA_Throw.IA_Throw"))
  (bind _ac_grabsystem (Variables|Default|GetAC_GrabSystem))
  ;[0.15 0.1095 0.01756 0.5] Grab System
  ;;[0.15 0.15 0.15 0.5] Input
  ;;;[1 0.6517 0.3191] Throw
  (:Started
    (Variables|/Game/GrabSystem/Blueprint/ActorComponent/AC_GrabSystem.AC_GrabSystem_C|GetAs%20BP%20Master%20Grab _ac_grabsystem
      (:then
        (Default|EndInteractServer _ac_grabsystem true (Variables|Default|GetQuickThrowPower)))
      (:else))))

(event EventBeginPlay
  (Class|ACInventory|StartComponent (Variables|Default|GetBP_AC_Inventory) false)
  (bind _returnvalue (UserInterface|CreateWidget "/IFP_CommonAssets/IFP_CommonAssets/Widgets/W_ControlsHUD.W_ControlsHUD_C"))
  (UserInterface|Viewport|AddtoViewport _returnvalue 0)
  (bind _returnvalue_2 (UserInterface|CreateWidget "/IFP_RPG/IFP_RPG/Widgets/QuickSlot/WBP_QuickSlotHUD.WBP_QuickSlotHUD_C"))
  (UserInterface|Viewport|AddtoViewport _returnvalue_2 0)
  (Default|InitializeSlots _returnvalue_2))

(event EventOnLanded
  (params (Hit :type Hit%20Result%20Structure%20%28by%20ref%29))
  ;[0.03432 0.15 0.1465 0.5] Movement
  (Default|OnLandedEvent (Variables|Default|GetAC_FPMovement) Hit))

(event EventOnWalkingOffLedge
  (params (PreviousFloorImpactNormal :type Vector%20%28by%20ref%29 :default "0, 0, 0") (PreviousFloorContactNormal :type Vector%20%28by%20ref%29 :default "0, 0, 0") (PreviousLocation :type Vector%20%28by%20ref%29 :default "0, 0, 0") (TimeDelta :type Float%20%28single-precision%29))
  ;[0.03432 0.15 0.1465 0.5] Movement
  (Default|OnWalkingOffLedgeEvent (Variables|Default|GetAC_FPMovement) PreviousFloorImpactNormal PreviousFloorContactNormal PreviousLocation TimeDelta))

(event EventTick
  (params (DeltaSeconds :type Float%20%28single-precision%29))
  ;[0.15 0.01837 0.007912 0.5] Begin Play and Tick
  (Variables|/FirstPersonMovementTemplate/Blueprints/BlueprintOnly/BP_BlueprintOnly_FPMovementComponent.BP_BlueprintOnly_FPMovementComponent_C|SetIA_Move_Value (Variables|Default|GetAC_FPMovement) (Input|EnhancedActionValues|GetIA_Move)))

(event EventSpawnActor
  (params (SpawnActorInfos :type F%20Spawn%20Actor%20Infos%20Structure))
  ;[0.15 0.1095 0.01756 0.5] Grab System
  ;;[1 0.6109 0.1818] Spawn actor logic
  (CallFunction|SpawnActorServer SpawnActorInfos))

(event Input|MouseEvents|MouseWheelAxis
  (params (AxisValue :type Float%20%28single-precision%29))
  ;[0.15 0.1095 0.01756 0.5] Grab System
  ;;[0.15 0.15 0.15 0.5] Input
  ;;;[1 0.6517 0.3191] Zoom in and out
  (if (!= AxisValue 0.0)
    (Default|ZoomOutin (Variables|Default|GetAC_GrabSystem) AxisValue)))

(event Input|KeyboardEvents|R
  (params (Key :type Key%20Structure :default "None"))
  (bind _ac_grabsystem (Variables|Default|GetAC_GrabSystem))
  ;[0.15 0.1095 0.01756 0.5] Grab System
  ;;[0.15 0.15 0.15 0.5] Input
  ;;;[1 0.6517 0.3191] Reset rotation
  (:Pressed
    (Variables|/Game/GrabSystem/Blueprint/ActorComponent/AC_GrabSystem.AC_GrabSystem_C|GetAs%20BP%20Master%20Grab _ac_grabsystem
      (:then
        (Default|ResetRotation _ac_grabsystem))
      (:else))))

(event Input|MouseEvents|MiddleMouseButton
  (params (Key :type Key%20Structure :default "None"))
  ;[0.15 0.1095 0.01756 0.5] Grab System
  ;;[0.15 0.15 0.15 0.5] Input
  ;;;[1 0.6517 0.3191] Limit Rotation Direction
  (:Pressed
    (CallFunction|LimitRotation))
  (:Released
    (CallFunction|UnlimitRotation)))

(event Input|KeyboardEvents|Q
  (params (Key :type Key%20Structure :default "None"))
  (bind _ac_grabsystem (Variables|Default|GetAC_GrabSystem))
  ;[0.15 0.1095 0.01756 0.5] Grab System
  ;;[0.15 0.15 0.15 0.5] Input
  ;;;[1 0.6517 0.3191] Rotate Grabbed Object
  (:Pressed
    (Variables|/Game/GrabSystem/Blueprint/ActorComponent/AC_GrabSystem.AC_GrabSystem_C|GetAs%20BP%20Master%20Grab _ac_grabsystem
      (:then
        (Default|RotationModeonOff _ac_grabsystem true))
      (:else)))
  (:Released
    (Variables|/Game/GrabSystem/Blueprint/ActorComponent/AC_GrabSystem.AC_GrabSystem_C|GetAs%20BP%20Master%20Grab _ac_grabsystem
      (:then
        (Default|RotationModeonOff _ac_grabsystem false))
      (:else))))

(fn ConstructionScript
  (Default|InitializeMovementSystem (Variables|Default|GetAC_FPMovement) self (Variables|Default|GetCameraSocket) (Variables|Default|GetCamera) (Variables|Default|GetInput%20Mapping%20Context))
  (Default|InitializeGrabSystem (Variables|Default|GetAC_GrabSystem) (Variables|Default|GetCamera) (Variables|Default|GetPhysicsHandle)))

(fn GetContainers
  (Development|PrintString "GetContainers( )")
  (bind _returnvalue (Class|ACInventory|GetAllContainerWidgets (Variables|Default|GetBP_AC_Inventory)))
  (return _returnvalue))

(fn GetInventoryComponent
  (return (Variables|Default|GetBP_AC_Inventory)))

(fn GetTriggerColliders
  (return (Variables|Default|GetTriggerRangeNear) (Variables|Default|GetTriggerRangeMid) (Variables|Default|GetTriggerRangeFar)))

(fn IsPreviewActor
  (return false))

(fn MeetsCurrencyCheck
  (params (Buyer :type AC%20Inventory%20Object%20Reference) (Currency :type IDA%20Currency%20Object%20Reference) (Amount :type Integer))
  (return false))

(fn MouseAxis
  (return (Variables|Default|GetTurn%20Axis%20Value) (Variables|Default|GetLookUp%20Axis%20Value)))