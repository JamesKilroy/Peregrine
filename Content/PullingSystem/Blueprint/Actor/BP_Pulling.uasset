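; Pulling cable actor that drags a physics-simulating component along the line from Point1 to Point2, managed by a pulling system component.
; Once readied, Tick applies an initial velocity, then repeated acceleration, or added velocity for cars, and forces net updates.
; Power comes from the target owner's BI_Pulling interface or defaults.
; It asks the system to destroy it within a threshold distance of Point2, unless disabled, or when the target becomes invalid.
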(event Custom|SetVeriables
  (params (AC_PullingSystem :type AC%20Pulling%20System%20Object%20Reference) (PrimitiveComp :type Primitive%20Component%20Object%20Reference))
  ;[1 0.6203 0.1906] Prepare Veriables
  (Variables|Other|SetAC_PullingSystem AC_PullingSystem)
  (bind _output_get (Variables|Other|SetPrimitiveComp PrimitiveComp))
  (if (Utilities|DoesObjectImplementInterface (Components|GetOwner _output_get) "/Game/PullingSystem/Blueprint/Interface/BI_Pulling.BI_Pulling_C")
    (bind _power (Class|BIPulling|PullingPower(Message) (Components|GetOwner _output_get)))
    (Variables|Pulling|SetPower _power)
    (elif (Variables|Other|GetIsCar)
      (Variables|Pulling|SetPower (Variables|Pulling|GetCarPower))
      (else
        (Variables|Pulling|SetPower 2e+03)))))

(event Custom|PreparePullingCollision
  (params (Enable%20Collision :type Boolean) (Collision%20Friction :type Float%20%28double-precision%29))
  (bind _cable (Variables|Components|GetCable))
  ;[1 0.6084 0.2014] Enable Collision
  (Variables|/Script/CableComponent.CableComponent|SetbEnableCollision _cable Enable%20Collision)
  (Variables|/Script/CableComponent.CableComponent|SetCollisionFriction _cable Collision%20Friction))

(event Custom|SetCompLocAndRot
  (bind _returnvalue (Utilities|Time|GetWorldDeltaSeconds))
  (bind _iscar (Variables|Other|GetIsCar))
  (bind _point1 (Variables|Components|GetPoint1))
  (bind _power (Variables|Pulling|GetPower))
  (bind _point2 (Variables|Components|GetPoint2))
  (bind _primitivecomp (Variables|Other|GetPrimitiveComp))
  (bind _power_2 (Variables|Pulling|GetPower))
  (bind _returnvalue_2 (Transformation|GetWorldLocation _point1))
  (bind _returnvalue_3 (Transformation|GetWorldLocation _point2))
  (bind _returnvalue_4 (* _returnvalue _power))
  (bind _returnvalue_5 (Math|Vector|GetUnitDirection(Vector) _returnvalue_2 _returnvalue_3))
  (bind _returnvalue_6 (Math|Float|SelectFloat _returnvalue_4 _power_2 _iscar))
  (bind _returnvalue_7 (* _returnvalue_5 _returnvalue_6))
  (bind (_x _y _z) (Math|Vector|BreakVector _returnvalue_7))
  ;[1 0.6203 0.1906] Add Force Multi
  (Utilities|FlowControl|Sequence
    (:then_0
      (Utilities|FlowControl|DoOnce false
        (:Completed
          (Class|PrimitiveComponent|SetAllPhysicsLinearVelocity (Variables|Other|GetPrimitiveComp) (* (Math|Vector|GetUnitDirection(Vector) (Transformation|GetWorldLocation (Variables|Components|GetPoint1)) (Transformation|GetWorldLocation (Variables|Components|GetPoint2))) 1e+02) false)
          (Variables|Default|SetDesiredDistance (Variables|Default|GetCurrentDistance)))))
    (:then_1
      (if (Variables|Other|GetIsCar)
        (Class|PrimitiveComponent|SetAllPhysicsLinearVelocity (Variables|Other|GetPrimitiveComp) _returnvalue_7 true)
        (else
          (Physics|AddForce _primitivecomp (Math|Vector|MakeVector _x _y _z) "None" true)))
      (Networking|ForceNetUpdate (Components|GetOwner _primitivecomp)))))

(event Custom|AddForceServer
  (bind _primitivecomp (Variables|Other|GetPrimitiveComp))
  (bind _point2 (Variables|Components|GetPoint2))
  (bind _returnvalue (Transformation|GetWorldLocation _primitivecomp))
  (bind _returnvalue_2 (Transformation|GetWorldLocation _point2))
  (bind _returnvalue_3 (Math|Vector|Distance(Vector) _returnvalue_2 _returnvalue))
  (bind _returnvalue_4 (/ _returnvalue_3 1e+02))
  ;[1 0.6203 0.1906] Add To Force Server
  (Variables|Other|GetAC_PullingSystem
    (:then
      (bind _primitivecomp_2 (Variables|Other|GetPrimitiveComp)
        (:then
          (if (Physics|IsSimulatingPhysics _primitivecomp_2 "None")
            (Variables|Default|SetCurrentDistance _returnvalue_4)
            (CallFunction|SetCompLocandRot)
            (if (and (<= _returnvalue_4 (Variables|Pulling|GetMaxDistanceForDestroy%28meter%29)) (not (Variables|Pulling|GetDisableMaxDistanceForDestroy)))
              (Default|DestroyPulling (Variables|Other|GetAC_PullingSystem) self :!label _label))))
        (:else
          (goto _label))))
    (:else
      (Actor|DestroyActor self))))

(event Custom|PreaprePulling
  (params (Enable%20Collision :type Boolean) (Collision%20Friction :type Float%20%28double-precision%29))
  ;[1 0.6203 0.1906] Set To Ready
  (CallFunction|PreparePullingCollision Enable%20Collision Collision%20Friction)
  (Variables|Other|SetIsItReady true)
  (Class|PrimitiveComponent|WakeAllRigidBodies (Variables|Other|GetPrimitiveComp)))

(event Custom|UpdateVariables
  (params (Power%20Value :type Float%20%28double-precision%29))
  ;[1 0.6203 0.1906] Prepare Veriables
)

(event EventTick
  (params (DeltaSeconds :type Float%20%28single-precision%29))
  ;[1 0.6203 0.1906] Event Tick
  (if (Variables|Other|GetIsItReady)
    (CallFunction|AddForceServer)))

(event Input|MouseEvents|MouseWheelAxis
  (params (AxisValue :type Float%20%28single-precision%29))
  (bind _output_get (Variables|Default|SetDesiredDistance (+ (Variables|Default|GetDesiredDistance) (* AxisValue 1.0))))
  (Development|PrintString (Utilities|String|ToString(Float) _output_get)))

(fn ConstructionScript)