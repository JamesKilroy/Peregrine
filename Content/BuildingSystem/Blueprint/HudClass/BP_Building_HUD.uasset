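; BP_Building_HUD is the building system's HUD, which draws a small crosshair icon at the screen's midpoint.
; DrawHUD picks the interact or non-interact texture from the Interact flag, which also selects the icon's size.
; The Crosshair flag gates which texture is supplied, and the icon's top-left corner sits at half the screen size, with no centering offset.
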(event EventDrawHUD
  (params (SizeX :type Integer) (SizeY :type Integer))
  (bind _interact (Variables|Default|GetInteract))
  (bind _returnvalue (Math|Float|SelectFloat 9.0 1e+01 _interact))
  (Canvas|DrawTexture (select (Variables|Default|GetCrosshair) (select (Variables|Default|GetInteract) "/Game/BuildingSystem/Texture/T_InteractIcon.T_InteractIcon" "/Game/BuildingSystem/Texture/T_NonInteractIcon.T_NonInteractIcon") 0) (Math|Conversions|ToFloat(Integer) (/ SizeX 2)) (Math|Conversions|ToFloat(Integer) (/ SizeY 2)) _returnvalue _returnvalue 0.0 0.0 1.0 1.0 "(R=1.000000,G=1.000000,B=1.000000,A=1.000000)"))

(fn ConstructionScript)